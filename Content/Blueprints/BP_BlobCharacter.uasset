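; Side-view player character for a blob platformer with swimming, an oxygen meter, a coin count and death with respawn at the start point.
; Tick switches between Flying and walking/falling from water-volume state, drains or refills oxygen and updates the HUD.
; Jump launches on land or triggers a cooldown-limited directional dash in water.
; Running out of oxygen triggers a timeline fade and respawn; HUD animations cycle texture arrays by sine of game time.
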(event Custom|KillEvent
  (Variables|Default|SetIsDead true)
  (Game|SpawnActorfromClass "/Game/Blueprints/BP_DeathEffectActor.BP_DeathEffectActor_C" (Math|Conversions|ToTransform(Vector) (Transformation|GetActorLocation)) "Undefined" 0 0)
  (Rendering|SetVisibility (Variables|Default|GetSprite) false false)
  (Input|DisableInput (Game|GetPlayerController 0))
  (Components|Activation|Deactivate (Variables|Character|GetCharacterMovement))
  (Variables|Default|SetOxygen 1e+02)
  (bind _newtrack_0 (Timeline|DeathTimeLine PlayFromStart)
    (:Update
      (Class|Image|SetOpacity (Variables|/Game/Blueprints/WG_GameHUD.WG_GameHUD_C|GetBlackImage (Variables|Default|GetHUD%20Ref)) _newtrack_0))
    (:NewTrack_1
      (CallFunction|RespawnEvent (Transformation|GetActorLocation)))))

(event Custom|RespawnEvent
  (params (NewLocation :type Vector))
  (Transformation|SetActorLocation (Variables|Default|GetSpawnLocation) false true)
  (Default|CheckifPlayerIsinWater (Variables|Default|GetWaterVolume_BP))
  (Variables|Default|SetOxygen 1e+02)
  (Variables|Default|SetIsDead false)
  (Rendering|SetVisibility (Variables|Default|GetSprite) true true)
  (Input|EnableInput (Game|GetPlayerController 0))
  (CallFunction|ResetUnderwaterKillDoOnce)
  (Components|Activation|Activate (Variables|Character|GetCharacterMovement) false)
  (Components|Movement|StopMovementImmediately (Variables|Character|GetCharacterMovement)))

(event Custom|ResetUnderwaterKillDoOnce
  (Utilities|FlowControl|DoOnce false) ; enters at Reset
)

(event Custom|ExitWaterEvent
  (bind _charactermovement (Variables|Character|GetCharacterMovement))
  (Variables|/Script/Engine.MovementComponent|SetVelocity _charactermovement (Math|Vector|ClampVectorSize (Variables|/Script/Engine.MovementComponent|GetVelocity _charactermovement) 0.0 1.2e+03)))

(event Custom|ResetDashDoOnce
  (Utilities|FlowControl|DoOnce false) ; enters at Reset
)

(event Custom|UpdateAnimation)

(event EventBeginPlay
  (Variables|Default|SetSpawnLocation (Transformation|GetActorLocation))
  (Variables|Default|SetCoinsCound 0)
  (Utilities|FlowControl|Sequence
    (:then_0
      (bind _returnvalue (UserInterface|CreateWidget "/Game/Blueprints/WG_GameHUD.WG_GameHUD_C"))
      (bind _output_get (Variables|Default|SetHUD%20Ref _returnvalue))
      (UserInterface|Viewport|AddtoViewport _output_get 0)
      (Variables|Default|SetOxygen 1e+02)
      (Variables|Default|SetIsDead false)
      (Variables|Default|SetSwimingDeceleration 6.5e+02))
    (:then_1
      (bind _outactors (Actor|GetAllActorsOfClass "/Game/Blueprints/BP_WaterVolume.BP_WaterVolume_C" :!label _label))
      (Utilities|IsValid (Utilities|Array|Get(acopy) _outactors)
        (:Is%20Valid
          (bind _output_get_2 (Variables|Default|SetWaterVolume_BP (Utilities|Array|Get(acopy) _outactors)))
          (Variables|Default|SetWaterHalfHeight (.z (Variables|/Script/Engine.BoxComponent|GetBoxExtent (Variables|/Game/Blueprints/BP_WaterVolume.BP_WaterVolume_C|GetTrigger _output_get_2))))
          (Default|CheckifPlayerIsinWater _output_get_2))
        (:Is%20Not%20Valid
          (Utilities|FlowControl|Delay 0.05)
          (goto _label))))))

(event EventTick
  (params (DeltaSeconds :type Float%20%28single-precision%29))
  (bind _returnvalue (Utilities|Time|GetWorldDeltaSeconds))
  (bind _charactermovement (Variables|Character|GetCharacterMovement))
  (bind _sprite (Variables|Default|GetSprite))
  (bind _swimingdeceleration (Variables|Default|GetSwimingDeceleration))
  (Default|UpdateProgressBar (Variables|Default|GetHUD%20Ref) (Variables|Default|GetOxygen))
  (Rendering|SetVisibility (Variables|Default|GetStaticMesh) (and (< (+ (.z (Transformation|GetActorLocation)) (Components|Capsule|GetScaledCapsuleHalfHeight (Variables|Collision|GetCapsuleComponent))) (+ (.z (Transformation|GetActorLocation (Variables|Default|GetWaterVolume_BP))) (Variables|Default|GetWaterHalfHeight))) (not (Variables|Default|GetIsDead))) false)
  (Rendering|Components|TextRender|SetText (Variables|/Game/Blueprints/WG_GameHUD.WG_GameHUD_C|GetScoreText (Variables|Default|GetHUD%20Ref)) (Utilities|Text|ToText(Integer) (Variables|Default|GetCoinsCound) false false))
  (if (Variables|Default|GetIsDead)
    (bind _currenttexture (CallFunction|PlayAnimation (Variables|Default|GetDeathAnimationArray) (Utilities|Time|GetGameTimeinSeconds) 2.0))
    (Appearance|SetBrushfromTexture (Variables|/Game/Blueprints/WG_GameHUD.WG_GameHUD_C|GetImage_63 (Variables|Default|GetHUD%20Ref)) _currenttexture false)
    (else
      (bind _currenttexture_2 (CallFunction|PlayAnimation (Variables|Default|GetProgressBarArray) (Utilities|Time|GetGameTimeinSeconds) 1.0))
      (Default|UpdateBreakBarTeture (Variables|Default|GetHUD%20Ref) _currenttexture_2)
      (bind _currenttexture_3 (CallFunction|PlayAnimation (Variables|Default|GetWakeUpArray) (Utilities|Time|GetGameTimeinSeconds) 1.0))
      (Appearance|SetBrushfromTexture (Variables|/Game/Blueprints/WG_GameHUD.WG_GameHUD_C|GetImage_63 (Variables|Default|GetHUD%20Ref)) _currenttexture_3 false)
      (Utilities|FlowControl|Sequence
        (:then_0
          (Math|Float|CompareFloat (.x (Variables|/Script/Engine.MovementComponent|GetVelocity (Variables|Character|GetCharacterMovement))) 0.0
            (:>
              (Transformation|SetWorldRotation _sprite "0,180.000000, 0" false false))
            (:<
              (Transformation|SetWorldRotation _sprite "0, 0, 0" false false))))
        (:then_1
          (Pawn|Input|AddMovementInput (Math|Vector|Normalize (Math|Vector|MakeVector (Input|AxisValues|GetMoveRight) 0.0 (select (Utilities|Enum|Equal(Enum) (Variables|/Script/Engine.CharacterMovementComponent|GetMovementMode (Variables|Character|GetCharacterMovement)) "MOVE_Flying") (Input|AxisValues|GetMoveUp) 0.0))) 1.0 false)
          (if (and (Utilities|Enum|Equal(Enum) (Variables|/Script/Engine.CharacterMovementComponent|GetMovementMode (Variables|Character|GetCharacterMovement)) "MOVE_Flying") (not (Variables|Default|GetIsDashing)))
            (Variables|/Script/Engine.CharacterMovementComponent|SetBrakingDecelerationFlying (Variables|Character|GetCharacterMovement) (select (> (Math|Vector|VectorLength (Variables|/Script/Engine.MovementComponent|GetVelocity _charactermovement)) (Variables|/Script/Engine.CharacterMovementComponent|GetMaxFlySpeed _charactermovement)) (* _swimingdeceleration 5.0) _swimingdeceleration))))
        (:then_2
          (if (and (Variables|Default|GetIsInsideWater) (not (Variables|Default|GetIsInsideFreeArea)))
            (if (< (.z (Transformation|GetActorLocation)) (+ (.z (Transformation|GetActorLocation (Variables|Default|GetWaterVolume_BP))) (Variables|Default|GetWaterHalfHeight)))
              (Pawn|Components|CharacterMovement|SetMovementMode (Variables|Character|GetCharacterMovement) "MOVE_Flying" 0))
            (else
              (Pawn|Components|CharacterMovement|SetMovementMode (Variables|Character|GetCharacterMovement) (select (.bblockinghit (Variables|/Script/Engine.CharacterMovementComponent|GetCurrentFloor (Variables|Character|GetCharacterMovement))) "MOVE_Walking" "MOVE_Falling") 0))))
        (:then_3
          (bind _output_get (Variables|Default|SetOxygen (Math|Float|Clamp(Float) (select (and (Utilities|Enum|Equal(Enum) (Variables|/Script/Engine.CharacterMovementComponent|GetMovementMode (Variables|Character|GetCharacterMovement)) "MOVE_Flying") (< (+ (.z (Transformation|GetActorLocation)) (Components|Capsule|GetScaledCapsuleHalfHeight (Variables|Collision|GetCapsuleComponent))) (+ (.z (Transformation|GetActorLocation (Variables|Default|GetWaterVolume_BP))) (Variables|Default|GetWaterHalfHeight)))) (+ (Variables|Default|GetOxygen) (* _returnvalue -4.0)) (+ (* _returnvalue 5e+01) (Variables|Default|GetOxygen))) 0.0 1e+02)))
          (if (<= _output_get 0.0)
            (Utilities|FlowControl|DoOnce false
              (:Completed
                (CallFunction|KillEvent)))))))))

(event Input|ActionEvents|InputActionJump
  (params (Key :type Key%20Structure))
  (:Pressed
    (if (Utilities|Enum|Equal(Enum) (Variables|/Script/Engine.CharacterMovementComponent|GetMovementMode (Variables|Character|GetCharacterMovement)) "MOVE_Flying")
      (Utilities|FlowControl|DoOnce false
        (:Completed
          (Audio|PlaySound2D "/Game/Assets/Audio/swinger_jump_02.swinger_jump_02" 1.0 1.0 0.0 0 0)
          (Variables|/Script/Engine.CharacterMovementComponent|SetBrakingDecelerationFlying (Variables|Character|GetCharacterMovement) 1e+03)
          (Variables|/Script/Engine.MovementComponent|SetVelocity (Variables|Character|GetCharacterMovement) (* (Math|Vector|Normalize (Math|Vector|MakeVector (Input|AxisValues|GetMoveRight) 0.0 (Input|AxisValues|GetMoveUp))) (Variables|Default|GetDashForce)))
          (Input|DisableInput (Game|GetPlayerController 0))
          (Variables|Default|SetIsDashing true)
          (Utilities|FlowControl|Delay 0.5)
          (Variables|Default|SetIsDashing false)
          (Input|EnableInput (Game|GetPlayerController 0))
          (Utilities|FlowControl|Delay 1.0)
          (CallFunction|ResetDashDoOnce)))
      (elif (AI|Components|NavMovement|IsMovingonGround (Variables|Character|GetCharacterMovement))
        (Character|LaunchCharacter (Math|Vector|MakeVector 0.0 0.0 (Math|Float|Sqrt (* (Math|Float|Absolute(Float) (Components|Movement|GetGravityZ (Variables|Character|GetCharacterMovement))) (Variables|Default|GetJumpHeight)))) false true)
        (Audio|PlaySound2D "/Game/Assets/Audio/swinger_jump_01.swinger_jump_01" 1.0 1.0 0.0 0 0)))))

(event Input|ActionEvents|InputActionAction
  (params (Key :type Key%20Structure))
  (:Pressed
    (if (not (Variables|Default|GetIsDead))
      (Default|HideMessage (Variables|Default|GetHUD%20Ref)))))

(fn ConstructionScript)

(fn PlayAnimation
  (params (Texture2DArray :type Array%20of%20Texture%202D%20Object%20References) (Time :type Float%20%28single-precision%29) (Rate :type Float%20%28single-precision%29))
  (return (Utilities|Array|Get(acopy) Texture2DArray (Math|Float|Truncate (* (Utilities|Array|LastIndex Texture2DArray) (Math|Float|Absolute(Float) (Math|Trig|Sin(Radians) (* Time Rate (Math|Trig|GetPI)))))))))