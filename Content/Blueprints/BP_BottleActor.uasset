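; BP_BottleActor is a pickup bottle that, when a BP_BlobCharacter overlaps its box, shows its configured message, optionally flagged as the end message, on that character's HUD.
; The bottle then destroys itself.
; Disconnected graphs hold unused buoyancy logic that would switch between Falling, Floating and Underwater using water and no-water volumes, physics, upward force and interpolation.
; BeginPlay and Tick are empty, so that logic never runs.
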(event OnComponentBeginOverlap(Box)
  (params (OverlappedComponent :type Primitive%20Component%20Object%20Reference) (OtherActor :type Actor%20Object%20Reference) (OtherComp :type Primitive%20Component%20Object%20Reference) (OtherBodyIndex :type Integer) (bFromSweep :type Boolean) (SweepResult :type Hit%20Result%20Structure%20%28by%20ref%29))
  (bind _asbp_blob_character (Utilities|Casting|CastToBP_BlobCharacter OtherActor))
  (Default|ShowMessage (Variables|/Game/Blueprints/BP_BlobCharacter.BP_BlobCharacter_C|GetHUD%20Ref _asbp_blob_character) (Variables|Default|GetMessage) (Variables|Default|GetIsEnd))
  (Actor|DestroyActor))

(event EventTick
  (params (DeltaSeconds :type Float%20%28single-precision%29)))

(event EventBeginPlay)

(fn ConstructionScript)