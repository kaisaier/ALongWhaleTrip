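; BP_JellyFishActor is a jellyfish hazard that patrols back and forth along a spline and kills the BP_BlobCharacter on contact.
; Tick eases speed toward a maximum, moves the sphere along the spline, and reverses direction with speed reset at each end.
; The sphere faces its travel direction, either instantly or interpolated, and its overlap calls KillEvent on a living blob.
; The construction script previews the starting position and orientation from CurrentDistance.
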(event OnComponentBeginOverlap(Sphere)
  (params (OverlappedComponent :type Primitive%20Component%20Object%20Reference) (OtherActor :type Actor%20Object%20Reference) (OtherComp :type Primitive%20Component%20Object%20Reference) (OtherBodyIndex :type Integer) (bFromSweep :type Boolean) (SweepResult :type Hit%20Result%20Structure%20%28by%20ref%29))
  (bind _asbp_blob_character (Utilities|Casting|CastToBP_BlobCharacter OtherActor))
  (if (not (Variables|/Game/Blueprints/BP_BlobCharacter.BP_BlobCharacter_C|GetIsDead _asbp_blob_character))
    (Default|KillEvent _asbp_blob_character)))

(event EventBeginPlay
  (Variables|Default|SetSplineLenght (Spline|GetSplineLength (Variables|Default|GetSpline))))

(event EventTick
  (params (DeltaSeconds :type Float%20%28single-precision%29))
  (bind _spline (Variables|Default|GetSpline))
  (Variables|Default|SetCurrentSpeed (Math|Interpolation|FInterpTo (Variables|Default|GetCurrentSpeed) (Variables|Default|GetMaxSpeed) DeltaSeconds (Variables|Default|GetSpeedInterpSpeed)))
  (bind _output_get (Variables|Default|SetCurrentDistance (Math|Float|Clamp(Float) (+ (Variables|Default|GetCurrentDistance) (* (Variables|Default|GetDirection) (Variables|Default|GetCurrentSpeed) DeltaSeconds)) 0.0 (Variables|Default|GetSplineLenght))))
  (Transformation|SetRelativeLocation (Variables|Default|GetSphere) (Spline|GetLocationatDistanceAlongSpline _spline _output_get "Local") false false)
  (Transformation|SetRelativeRotation (Variables|Default|GetSphere) (select (Variables|Default|GetIsInstantRotation) (Math|Conversions|RotationFromXVector (* (Spline|GetTangentatDistanceAlongSpline _spline _output_get "Local") (Variables|Default|GetDirection))) (Math|Interpolation|RInterpTo (Variables|/Script/Engine.SceneComponent|GetRelativeRotation (Variables|Default|GetSphere)) (Math|Conversions|RotationFromXVector (* (Spline|GetTangentatDistanceAlongSpline _spline _output_get "Local") (Variables|Default|GetDirection))) (Utilities|Time|GetWorldDeltaSeconds) (Variables|Default|GetRotationInterpSpeed))) false false)
  (if (>= (Variables|Default|GetCurrentDistance) (Variables|Default|GetSplineLenght))
    (Variables|Default|SetDirection -1.0)
    (Variables|Default|SetCurrentSpeed 0.0 :!label _label)
    (elif (<= (Variables|Default|GetCurrentDistance) 0.0)
      (Variables|Default|SetDirection 1.0)
      (goto _label))))

(fn ConstructionScript
  (bind _spline (Variables|Default|GetSpline))
  (bind _output_get (Variables|Default|SetCurrentDistance (Math|Float|Clamp(Float) (Variables|Default|GetCurrentDistance) 0.0 (Spline|GetSplineLength (Variables|Default|GetSpline)))))
  (Transformation|SetRelativeLocation (Variables|Default|GetSphere) (Spline|GetLocationatDistanceAlongSpline _spline _output_get "Local") false false)
  (Transformation|SetRelativeRotation (Variables|Default|GetSphere) (Math|Conversions|RotationFromXVector (* (Spline|GetTangentatDistanceAlongSpline _spline _output_get "Local") (Variables|Default|GetDirection))) false false))