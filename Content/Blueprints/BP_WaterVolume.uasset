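; BP_WaterVolume is a water trigger volume that flags bottles and the blob character as in or out of water.
; Overlap events set those flags, and a blob leaving the water also gets its exit event called.
; When the volume is not moving, blob crossings spawn a splash at the box's top height, and entry also cuts the blob's velocity to a quarter.
; A separate event re-syncs the player's water flag from current overlaps.
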(event OnComponentBeginOverlap(Trigger)
  (params (OverlappedComponent :type Primitive%20Component%20Object%20Reference) (OtherActor :type Actor%20Object%20Reference) (OtherComp :type Primitive%20Component%20Object%20Reference) (OtherBodyIndex :type Integer) (bFromSweep :type Boolean) (SweepResult :type Hit%20Result%20Structure%20%28by%20ref%29))
  (bind _asbp_bottle_actor (Utilities|Casting|CastToBP_BottleActor OtherActor)
    (:then
      (Variables|/Game/Blueprints/BP_BottleActor.BP_BottleActor_C|SetIsInWater _asbp_bottle_actor true))
    (:CastFailed
      (bind _asbp_blob_character (Utilities|Casting|CastToBP_BlobCharacter OtherActor))
      (Variables|/Game/Blueprints/BP_BlobCharacter.BP_BlobCharacter_C|SetIsInsideWater _asbp_blob_character true)
      (if (not (Variables|Default|GetIsMoving))
        (Game|SpawnActorfromClass "/Game/Blueprints/BP_SplashActor.BP_SplashActor_C" (Math|Transform|MakeTransform (Math|Vector|MakeVector (.x (Transformation|GetActorLocation _asbp_blob_character)) (.y (Transformation|GetActorLocation _asbp_blob_character)) (+ (.z (Variables|/Script/Engine.BoxComponent|GetBoxExtent (Variables|Default|GetTrigger))) (.z (Transformation|GetActorLocation)))) "0, 0, 0" "1,1,1") "Undefined" 0 0)
        (Variables|/Script/Engine.MovementComponent|SetVelocity (Variables|/Script/Engine.Character|GetCharacterMovement _asbp_blob_character) (/ (Variables|/Script/Engine.MovementComponent|GetVelocity (Variables|/Script/Engine.Character|GetCharacterMovement _asbp_blob_character)) 4.0))))))

(event OnComponentEndOverlap(Trigger)
  (params (OverlappedComponent :type Primitive%20Component%20Object%20Reference) (OtherActor :type Actor%20Object%20Reference) (OtherComp :type Primitive%20Component%20Object%20Reference) (OtherBodyIndex :type Integer))
  (bind _asbp_bottle_actor (Utilities|Casting|CastToBP_BottleActor OtherActor)
    (:then
      (Variables|/Game/Blueprints/BP_BottleActor.BP_BottleActor_C|SetIsInWater _asbp_bottle_actor false))
    (:CastFailed
      (bind _asbp_blob_character (Utilities|Casting|CastToBP_BlobCharacter OtherActor))
      (Variables|/Game/Blueprints/BP_BlobCharacter.BP_BlobCharacter_C|SetIsInsideWater _asbp_blob_character false)
      (Default|ExitWaterEvent _asbp_blob_character)
      (if (not (Variables|Default|GetIsMoving))
        (Game|SpawnActorfromClass "/Game/Blueprints/BP_SplashActor.BP_SplashActor_C" (Math|Transform|MakeTransform (Math|Vector|MakeVector (.x (Transformation|GetActorLocation _asbp_blob_character)) (.y (Transformation|GetActorLocation _asbp_blob_character)) (+ (.z (Variables|/Script/Engine.BoxComponent|GetBoxExtent (Variables|Default|GetTrigger))) (.z (Transformation|GetActorLocation)))) "0, 0, 0" "1,1,1") "Undefined" 0 0)))))

(event Custom|CheckIfPlayerIsInWater
  (bind _asbp_blob_character (Utilities|Casting|CastToBP_BlobCharacter (Game|GetPlayerCharacter 0)))
  (Variables|/Game/Blueprints/BP_BlobCharacter.BP_BlobCharacter_C|SetIsInsideWater _asbp_blob_character (Utilities|Array|ContainsItem (Collision|GetOverlappingActors (Variables|Default|GetTrigger) "/Game/Blueprints/BP_BlobCharacter.BP_BlobCharacter_C" :!class /Script/Engine.PrimitiveComponent) (Game|GetPlayerCharacter 0))))

(fn ConstructionScript)