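; BP_CoinActor is a coin pickup that the blob character collects by touching it.
; It keeps overlap events on its Sphere off for a short delay after BeginPlay, then turns them on.
; An overlap with a BP_BlobCharacter increments that character's CoinsCound counter, plays a 2D coin sound and destroys the coin.
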(event OnComponentBeginOverlap(Sphere)
  (params (OverlappedComponent :type Primitive%20Component%20Object%20Reference) (OtherActor :type Actor%20Object%20Reference) (OtherComp :type Primitive%20Component%20Object%20Reference) (OtherBodyIndex :type Integer) (bFromSweep :type Boolean) (SweepResult :type Hit%20Result%20Structure%20%28by%20ref%29))
  (bind _asbp_blob_character (Utilities|Casting|CastToBP_BlobCharacter OtherActor))
  (Math|Integer|IncrementInt (Variables|/Game/Blueprints/BP_BlobCharacter.BP_BlobCharacter_C|GetCoinsCound _asbp_blob_character)
    (:%20%20
      (Audio|PlaySound2D "/Game/Assets/Audio/Swinger_CoinSound_Cue.Swinger_CoinSound_Cue" 1.0 1.0 0.0 0 0)
      (Actor|DestroyActor))))

(event EventBeginPlay
  (Variables|/Script/Engine.PrimitiveComponent|SetbGenerateOverlapEvents (Variables|Default|GetSphere) false)
  (Utilities|FlowControl|Delay 0.5)
  (Variables|/Script/Engine.PrimitiveComponent|SetbGenerateOverlapEvents (Variables|Default|GetSphere) true))

(fn ConstructionScript)